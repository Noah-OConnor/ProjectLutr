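; BP_WeaponBase is a base weapon driven by WeaponData, handling capacity-limited firing.
; Initialize stores the data and starting capacity, then applies any valid mesh and material to the skeletal WeaponMesh.
; TryFireWeapon checks capacity against the fire cost before FireWeapon deducts it, prints a debug string and calls the OnWeaponFire dispatcher.
; Reload is an empty stub, and no projectile or damage logic exists here.
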(fn `FireWeapon`
  (bind (_weapondata_name _weapondata_firerate _weapondata_maxcapacity _weapondata_firecapacitycost) (break `/Game/F_WeaponData` (`self.WeaponData`)))
  (set `self.CurrentCapacity` (- (`self.CurrentCapacity`) _weapondata_firecapacitycost))
  (`KismetSystemLibrary.PrintString` "FireWeapon")
  (`self.OnWeaponFire`))

(fn `Initialize`
  (params (WeaponData :type "/Game/F_WeaponData Structure") (CurrentCapacity :type "Float (double-precision)"))
  (bind (_weapondata_name _weapondata_firerate _weapondata_maxcapacity _weapondata_firecapacitycost _weapondata_spread _weapondata_fireabilityclass _weapondata_fireabiltiytag _weapondata_projectileclass _weapondata_staticmesh _weapondata_material) (break `/Game/F_WeaponData` (`self.WeaponData`)))
  (set `self.WeaponData` WeaponData)
  (set `self.CurrentCapacity` CurrentCapacity)
  (`/Engine/EditorBlueprintResources/StandardMacros.IsValid` _weapondata_staticmesh
    (:`Is Valid`
      (`SkeletalMeshComponent.SetSkeletalMeshAsset` (`self.WeaponMesh`) _weapondata_staticmesh))
    (:`Is Not Valid`
      _))
  (`/Engine/EditorBlueprintResources/StandardMacros.IsValid` _weapondata_material
    (:`Is Valid`
      (`PrimitiveComponent.SetMaterial` (`self.WeaponMesh`) 0 _weapondata_material))))

(fn `Reload`)

(fn `TryFireWeapon`
  (bind (_weapondata_name _weapondata_firerate _weapondata_maxcapacity _weapondata_firecapacitycost) (break `/Game/F_WeaponData` (`self.WeaponData`)))
  (if (>= (`self.CurrentCapacity`) _weapondata_firecapacitycost)
    (`self.FireWeapon`)))

(fn `UserConstructionScript`)