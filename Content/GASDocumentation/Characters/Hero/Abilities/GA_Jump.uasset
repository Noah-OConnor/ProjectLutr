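; GA_Jump is a Gameplay Ability that makes the avatar Character jump.
; Activation is only allowed when the character's movement component is not falling, so there is no jumping in midair.
; On activation it commits the ability cost, calls Jump and ends immediately, or cancels if the commit fails.
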(event `self.K2_ActivateAbility`
  ;[0 0 1] Commit ability cost
  (bind _returnvalue (`self.K2_CommitAbility`))
  (if _returnvalue
    (bind _ascharacter (cast `Character` (`self.GetAvatarActorFromActorInfo`)))
    (`Character.Jump` _ascharacter)
    (`self.K2_EndAbility`)
    (else
      (`self.K2_CancelAbility`) ; Couldn't afford ability cost, cancel ability.
    )))

(fn `K2_CanActivateAbility`
  (params (ActorInfo :type "GameplayAbilityActorInfo Structure") (Handle :type "GameplayAbilitySpecHandle Structure"))
  (returns (RelevantTags :type "GameplayTagContainer Structure") (ReturnValue :type Boolean))
  (bind _ascharacter (cast `Character` (`self.GetAvatarActorFromActorInfo`)))
  (return (struct) (not (`NavMovementInterface.IsFalling` (`Character.CharacterMovement` _ascharacter)))))