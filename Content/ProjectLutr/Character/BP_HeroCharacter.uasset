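; First-person hero character that adds the HUD and drives jumping, abilities and weapons through the Gameplay Ability System.
; Test keys stage an ability, then a slot key grants and binds its tag for later activation.
; Equipping spawns an inventory weapon on the first-person mesh and grants its fire ability.
; The weapon's fire callback sends a gameplay event carrying camera and muzzle transforms in a payload object.
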(event `self.ReceiveBeginPlay`
  (bind _returnvalue (`|CreateWidget` "/Game/ProjectLutr/UI/BP_HUD.BP_HUD_C"))
  (`UserWidget.AddToViewport` _returnvalue 0))

(event `Key|SpaceBar`
  (params (Key :type "Key Structure"))
  ;[1 0.9564 0.2604 0.5] Jumping
  (:`Pressed`
    (`AbilitySystemComponent.TryActivateAbilitiesByTag` (`AbilitySystemBlueprintLibrary.GetAbilitySystemComponent` null) (`BlueprintGameplayTagLibrary.MakeGameplayTagContainerFromTag` (struct :`TagName` "Ability.Jump")) true)))

(event `Key|Four`
  (params (Key :type "Key Structure"))
  (bind _weaponsininventory (`self.WeaponsInInventory`))
  (:`Pressed`
    (if (`KismetArrayLibrary.Array_IsNotEmpty` _weaponsininventory)
      (`self.EquipWeapon` (`|GetArrayItem` _weaponsininventory))
      (add `/Game/ProjectLutr/Blueprints/BP_WeaponBase.OnWeaponFire` (`self.Active Weapon`) (delegate `OnWeaponFire`)))))

(event `Key|One`
  (params (Key :type "Key Structure"))
  ;[0.05729 0 0] Ability Slot Testing
  (:`Pressed`
    (if (`self.bTryAssignTag`)
      (set `self.Slot1Tag` (`self.TagToAssign`))
      (set `self.TagToAssign` (struct))
      (`self.AssignAbilityToSlot`)
      (elif (not (== (`self.Slot1Tag`) (`BlueprintGameplayTagLibrary.MakeGameplayTagContainerFromTag` (struct))))
        (`AbilitySystemComponent.TryActivateAbilitiesByTag` (`AbilitySystemBlueprintLibrary.GetAbilitySystemComponent` null) (`self.Slot1Tag`) true)))))

(event `Key|LeftMouseButton`
  (params (Key :type "Key Structure"))
  (bind _active_weapon (`self.Active Weapon`))
  (:`Pressed`
    (`/Engine/EditorBlueprintResources/StandardMacros.IsValid` _active_weapon
      (:`Is Valid`
        (`/Game/ProjectLutr/Blueprints/BP_WeaponBase.TryFireWeapon` _active_weapon)))))

(event `OnWeaponFire`
  (bind _weaponfirepayload (`self.WeaponFirePayload`))
  (bind _active_weapon (`self.Active Weapon`))
  (bind (_weapondata_name _weapondata_firerate _weapondata_maxcapacity _weapondata_firecapacitycost _weapondata_spread _weapondata_fireabilityclass _weapondata_fireabiltiytag) (break `/Game/ProjectLutr/Blueprints/Data/F_WeaponData` (`/Game/ProjectLutr/Blueprints/BP_WeaponBase.WeaponData` _active_weapon)))
  (bind _returnvalue (`|GenericCreateObject` "/Game/ProjectLutr/Blueprints/AbilityPayloads/BP_WeaopnFirePayload.BP_WeaopnFirePayload_C"))
  (set `self.WeaponFirePayload` _returnvalue)
  (set `/Game/ProjectLutr/Blueprints/AbilityPayloads/BP_WeaopnFirePayload.CameraTransform` (`SceneComponent.K2_GetComponentToWorld` (`self.Camera`)) _weaponfirepayload)
  (set `/Game/ProjectLutr/Blueprints/AbilityPayloads/BP_WeaopnFirePayload.SpawnTransform` (`SceneComponent.GetSocketTransform` (`/Game/ProjectLutr/Blueprints/BP_WeaponBase.WeaponMesh` _active_weapon) "Muzzle" "RTS_World") _weaponfirepayload)
  (`AbilitySystemBlueprintLibrary.SendGameplayEventToActor` (`ActorComponent.GetOwner` (`AbilitySystemBlueprintLibrary.GetAbilitySystemComponent` null)) (`|GetArrayItem` (`BlueprintGameplayTagLibrary.BreakGameplayTagContainer` _weapondata_fireabiltiytag)) (make `GameplayEventData` (struct) null null (`self.WeaponFirePayload`))))

(event `Key|Two`
  (params (Key :type "Key Structure"))
  ;[0.05729 0 0] Ability Slot Testing
  (:`Pressed`
    (if (`self.bTryAssignTag`)
      (set `self.Slot2Tag` (`self.TagToAssign`))
      (set `self.TagToAssign` (struct))
      (`self.AssignAbilityToSlot`)
      (elif (not (== (`self.Slot2Tag`) (`BlueprintGameplayTagLibrary.MakeGameplayTagContainerFromTag` (struct))))
        (`AbilitySystemComponent.TryActivateAbilitiesByTag` (`AbilitySystemBlueprintLibrary.GetAbilitySystemComponent` null) (`self.Slot2Tag`) true)))))

(event `Key|Three`
  (params (Key :type "Key Structure"))
  ;[0.05729 0 0] Ability Slot Testing
  (:`Pressed`
    (if (`self.bTryAssignTag`)
      (set `self.Slot3Tag` (`self.TagToAssign`))
      (set `self.TagToAssign` (struct))
      (`self.AssignAbilityToSlot`)
      (elif (not (== (`self.Slot3Tag`) (`BlueprintGameplayTagLibrary.MakeGameplayTagContainerFromTag` (struct))))
        (`AbilitySystemComponent.TryActivateAbilitiesByTag` (`AbilitySystemBlueprintLibrary.GetAbilitySystemComponent` null) (`self.Slot3Tag`) true)))))

(event `Key|Z`
  (params (Key :type "Key Structure"))
  ;[0.05729 0 0] Ability Slot Testing
  (:`Pressed`
    (set `self.bTryAssignTag` true)
    (set `self.TagToAssign` (`self.AbilityAlphaTag`))
    (set `self.AbilityToGive` (`self.AbilityAlphaClass`))
    (`KismetSystemLibrary.PrintString` "Initiated Assigning Ability Alpha")))

(event `Key|X`
  (params (Key :type "Key Structure"))
  ;[0.05729 0 0] Ability Slot Testing
  (:`Pressed`
    (set `self.bTryAssignTag` true)
    (set `self.TagToAssign` (`self.AbilityBetaTag`))
    (set `self.AbilityToGive` (`self.AbilityBetaClass`))
    (`KismetSystemLibrary.PrintString` "Initiated Assigning Ability Beta")))

(event `Key|C`
  (params (Key :type "Key Structure"))
  ;[0.05729 0 0] Ability Slot Testing
  (:`Pressed`
    (set `self.bTryAssignTag` true)
    (set `self.TagToAssign` (`self.AbilityCharlieTag`))
    (set `self.AbilityToGive` (`self.AbilityCharlieClass`))
    (`KismetSystemLibrary.PrintString` "Initiated Assigning Ability Charlie")))

(fn `AssignAbilityToSlot`
  (set `self.bTryAssignTag` false)
  (`AbilitySystemComponent.K2_GiveAbility` (`AbilitySystemBlueprintLibrary.GetAbilitySystemComponent` null) (`self.AbilityToGive`) 0 -1)
  (set `self.AbilityToGive` null)
  (`KismetSystemLibrary.PrintString` (`KismetStringLibrary.Concat_StrStr` "Assigned Ability to " "Slot")))

(fn `EquipWeapon`
  (params (WeaponInstance :type "/Game/ProjectLutr/Blueprints/Data/F_WeaponInstance Structure"))
  (bind _weaponinstance_weaponclass (break `/Game/ProjectLutr/Blueprints/Data/F_WeaponInstance` (`local.WeaponInstance`)))
  (bind (_weaponinstance_weaponclass_2 _weaponinstance_weapondata _weaponinstance_currentcapacity) (break `/Game/ProjectLutr/Blueprints/Data/F_WeaponInstance` (`local.WeaponInstance`)))
  (`/Engine/EditorBlueprintResources/StandardMacros.IsValid` (`self.Active Weapon`)
    (:`Is Valid`
      (`self.K2_DestroyActor` (`self.Active Weapon`)))
    (:`Is Not Valid`
      _))
  (bind _returnvalue (`|SpawnActorFromClass` _weaponinstance_weaponclass (`self.GetTransform`) "Undefined" "MultiplyWithRoot" null null))
  (bind _output_get (set `self.Active Weapon` _returnvalue))
  (`self.K2_AttachToComponent` _output_get (`self.FirstPersonMesh`) "GripPoint" "SnapToTarget" "SnapToTarget" "SnapToTarget" true)
  (`/Game/ProjectLutr/Blueprints/BP_WeaponBase.Initialize` (`self.Active Weapon`) _weaponinstance_weapondata _weaponinstance_currentcapacity)
  (`AbilitySystemComponent.K2_GiveAbility` (`AbilitySystemBlueprintLibrary.GetAbilitySystemComponent` null) (`.FireAbilityClass_50_4D437B21404DDCADD2009B903AF86D85` (break `/Game/ProjectLutr/Blueprints/Data/F_WeaponData` (`.WeaponData_35_A68CF38A4E2B9F30D68D85BACE4E0213` (break `/Game/ProjectLutr/Blueprints/Data/F_WeaponInstance` (`local.WeaponInstance`))))) 0 -1)
  (`KismetArrayLibrary.Array_RemoveItem` (`self.WeaponsInInventory`) (`local.WeaponInstance`)))

(fn `UserConstructionScript`)