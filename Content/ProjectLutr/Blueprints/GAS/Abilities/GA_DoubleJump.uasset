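; Gameplay ability intended as a character double jump.
; Its activation check passes only while the avatar Character is falling with jumps left below its maximum, and prints a message if the cast fails.
; ActivateAbility is empty: the commit, Jump and end-or-cancel logic exists in the event graph but is disconnected, so this Blueprint's graph performs no jump.
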(event `self.K2_ActivateAbility`)

(fn `K2_CanActivateAbility`
  (params (ActorInfo :type "GameplayAbilityActorInfo Structure") (Handle :type "GameplayAbilitySpecHandle Structure"))
  (returns (RelevantTags :type "GameplayTagContainer Structure") (ReturnValue :type Boolean))
  (bind _ascharacter (cast `Character` (`self.GetAvatarActorFromActorInfo`))
    (:`then`
      (return (struct) (and (`NavMovementInterface.IsFalling` (`Character.CharacterMovement` _ascharacter)) (< (`Character.JumpCurrentCount` _ascharacter) (`Character.JumpMaxCount` _ascharacter)))))
    (:`CastFailed`
      (`KismetSystemLibrary.PrintString` "cast failed"))))