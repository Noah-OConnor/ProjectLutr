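; GA_EquipWeapon is a gameplay ability that equips the hero character's first inventory weapon, acting only with authority.
; It destroys any active weapon, spawns the new one on the first-person mesh's GripPoint socket, and initializes it from WeaponData and saved capacity.
; It then binds the player's HUD to the weapon, grants that weapon's fire and reload abilities, and ends.
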(event `self.K2_ActivateAbility`
  (bind _bpcharacter (`self.BPCharacter`))
  (bind _bpcharacter_2 (`self.BPCharacter`))
  (bind _bpcharacter_3 (`self.BPCharacter`))
  (bind _active_weapon (`/Game/ProjectLutr/Blueprints/Character/BP_HeroCharacter.Active Weapon` (`self.BPCharacter`)))
  (bind (_output_weaponname _output_weaponclass _output_currentcapacity) (break `/Game/ProjectLutr/Blueprints/Data/F_WeaponInstance` (`|GetArrayItem` (`/Game/ProjectLutr/Blueprints/Character/BP_HeroCharacter.InventoryWeaponInstances` (`self.BPCharacter`)))))
  (bind (_output_weaponname_2 _output_weaponclass_2) (break `/Game/ProjectLutr/Blueprints/Data/F_WeaponInstance` (`|GetArrayItem` (`/Game/ProjectLutr/Blueprints/Character/BP_HeroCharacter.InventoryWeaponInstances` (`self.BPCharacter`)))))
  (bind (_weapondata_name _weapondata_firerate _weapondata_maxcapacity _weapondata_firecapacitycost _weapondata_spread _weapondata_fireweaponabilityclass _weapondata_reloadweaponabilityclass) (break `/Game/ProjectLutr/Blueprints/Data/F_WeaponData` (`/Game/ProjectLutr/Blueprints/BP_WeaponBase.WeaponData` (`/Game/ProjectLutr/Blueprints/Character/BP_HeroCharacter.Active Weapon` (`self.BPCharacter`)))))
  (`self.K2_HasAuthority`
    (:`True`
      (`KismetSystemLibrary.PrintString` "Equip Weapno Called")
      (bind _asbp_hero_character (cast `/Game/ProjectLutr/Blueprints/Character/BP_HeroCharacter` (`self.GetAvatarActorFromActorInfo`))
        (:`then`
          (set `self.BPCharacter` _asbp_hero_character)
          (`/Engine/EditorBlueprintResources/StandardMacros.IsValid` _active_weapon
            (:`Is Valid`
              (`Actor.K2_DestroyActor` _active_weapon))
            (:`Is Not Valid`
              _))
          (bind _returnvalue (`|SpawnActorFromClass` _output_weaponclass_2 (`Actor.GetTransform` (`self.BPCharacter`)) "Undefined" "MultiplyWithRoot" _bpcharacter_2 _bpcharacter_2))
          (set `/Game/ProjectLutr/Blueprints/Character/BP_HeroCharacter.Active Weapon` _returnvalue _bpcharacter)
          (`Actor.K2_AttachToComponent` (`/Game/ProjectLutr/Blueprints/Character/BP_HeroCharacter.Active Weapon` _bpcharacter) (`/Game/ProjectLutr/Blueprints/Character/BP_HeroCharacter.FirstPersonMesh` _bpcharacter) "GripPoint" "SnapToTarget" "SnapToTarget" "SnapToTarget" true)
          (`/Game/ProjectLutr/Blueprints/BP_WeaponBase.Initialize` (`/Game/ProjectLutr/Blueprints/Character/BP_HeroCharacter.Active Weapon` (`self.BPCharacter`)) (`BlueprintMapLibrary.Map_Find` (`/Game/ProjectLutr/Blueprints/Data/BP_WeaponData.WeaponMap` (`/Game/ProjectLutr/Blueprints/Character/BP_HeroCharacter.WeaponData` (`self.BPCharacter`))) _output_weaponname) _output_currentcapacity)
          (`self.BindUI`)
          (`KismetSystemLibrary.PrintString` "Giving Weapon Abilities")
          (`/Game/ProjectLutr/Blueprints/Character/BP_HeroCharacter.GiveAbility` _bpcharacter_3 _weapondata_fireweaponabilityclass)
          (`/Game/ProjectLutr/Blueprints/Character/BP_HeroCharacter.GiveAbility` _bpcharacter_3 _weapondata_reloadweaponabilityclass)
          (`self.K2_EndAbility`))
        (:`CastFailed`
          (`KismetSystemLibrary.PrintString` "Failed cast to BP Hero"))))
    (:`False`
      (`KismetSystemLibrary.PrintString` "don't have authority"))))

(event `BindUI`
  ; Bind Weapon Ammo UI event
  (bind _asbp_player_controller (cast `/Game/ProjectLutr/Blueprints/BP_PlayerController` (`Pawn.GetController` (`self.BPCharacter`)))
    (:`then`
      (bind _aswbp_hud (cast `/Game/ProjectLutr/Blueprints/UI/WBP_HUD` (`GDPlayerController.UIHUDWidget` _asbp_player_controller))
        (:`then`
          (`/Game/ProjectLutr/Blueprints/UI/WBP_HUD.BindToCurrentWeapon` _aswbp_hud (`/Game/ProjectLutr/Blueprints/Character/BP_HeroCharacter.Active Weapon` (`self.BPCharacter`))))
        (:`CastFailed`
          (`KismetSystemLibrary.PrintString` "FAILED CAST TO WBP_HUD"))))
    (:`CastFailed`
      (`KismetSystemLibrary.PrintString` "FAILED CAST TO BP_PLAYERCONTROLLER"))))