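; GA_FireWeapon is a gameplay ability that resolves a weapon shot from the hit result carried in its triggering event's target data.
; On authority it spawns BP_Projectile at the impact point, or at the trace end on a miss, with debug prints.
; A hit actor's ability system component creates and self-applies GE_Damage with a fixed SetByCaller amount.
; The non-authority branch only prints and never ends the ability.
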(event `self.K2_ActivateAbilityFromEvent`
  (params (EventData :type "GameplayEventData Structure (by ref)"))
  (bind (_returnvalue_bblockinghit _returnvalue_binitialoverlap _returnvalue_time _returnvalue_distance _returnvalue_location _returnvalue_impactpoint _returnvalue_normal _returnvalue_impactnormal _returnvalue_physmat _returnvalue_hitactor _returnvalue_hitcomponent _returnvalue_hitbonename _returnvalue_bonename _returnvalue_hititem _returnvalue_elementindex _returnvalue_faceindex _returnvalue_tracestart _returnvalue_traceend) (`GameplayStatics.BreakHitResult` (`AbilitySystemBlueprintLibrary.GetHitResultFromTargetData` EventData_TargetData)))
  (bind _returnvalue (`KismetSystemLibrary.GetDisplayName` _returnvalue_hitactor))
  (bind _returnvalue_2 (`AbilitySystemBlueprintLibrary.GetAbilitySystemComponent` _returnvalue_hitactor))
  (`self.K2_HasAuthority`
    (:`True`
      (`KismetSystemLibrary.PrintString` "Actiavte Ability Fire Weapon")
      (if (`AbilitySystemBlueprintLibrary.TargetDataHasHitResult` EventData_TargetData)
        (set `self.HitLocation` _returnvalue_location)
        (`KismetSystemLibrary.PrintString` (`KismetStringLibrary.Concat_StrStr` "Hit " _returnvalue " in " (`KismetSystemLibrary.GetDisplayName` _returnvalue_hitcomponent)))
        (else
          (set `self.HitLocation` _returnvalue_traceend)
          (`KismetSystemLibrary.PrintString` "Hit Nothing")))
      (`|SpawnActorFromClass` "/Game/ProjectLutr/Blueprints/BP_Projectile.BP_Projectile_C" (`KismetMathLibrary.MakeTransform` (`self.HitLocation`)) "Undefined" "MultiplyWithRoot" null 0.0 (struct) null)
      (`KismetSystemLibrary.PrintString` (`KismetStringLibrary.Concat_StrStr` _returnvalue "has ASC"))
      (`/Engine/EditorBlueprintResources/StandardMacros.IsValid` _returnvalue_2
        (:`Is Valid`
          (bind _returnvalue_3 (`AbilitySystemBlueprintLibrary.AssignTagSetByCallerMagnitude` (`AbilitySystemComponent.MakeOutgoingSpec` :`self` _returnvalue_2 :`GameplayEffectClass` "/Game/ProjectLutr/Blueprints/GAS/Effects/GE_Damage.GE_Damage_C" :`Level` 1.0) (struct :`TagName` "SetByCallerTags.DamageAmount") 10.0))
          (`AbilitySystemComponent.BP_ApplyGameplayEffectSpecToSelf` _returnvalue_2 _returnvalue_3)
          (`self.K2_EndAbility`))
        (:`Is Not Valid`
          (`self.K2_EndAbility`))))
    (:`False`
      (`KismetSystemLibrary.PrintString` "Done's Have Authority"))))