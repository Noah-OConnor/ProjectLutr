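; Gameplay ability that reloads the hero character's active weapon from their ammo reserve.
; On activation it takes the lesser of the missing capacity and the reserve, then passes the new total to the weapon's Reload.
; It deducts that amount from the reserve attribute by applying GE_ConsumeAmmoResreve with a negative SetByCaller magnitude.
; EndAbility is called only when a reload happens, not on the failed-check paths.
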(event `self.K2_ActivateAbility`
  (`KismetSystemLibrary.PrintString` "Called GA Relaod Weapno")
  (bind _asbp_hero_character (cast `/Game/ProjectLutr/Blueprints/Character/BP_HeroCharacter` (`self.GetAvatarActorFromActorInfo`))
    (:`then`
      (bind _active_weapon (`/Game/ProjectLutr/Blueprints/Character/BP_HeroCharacter.Active Weapon` _asbp_hero_character))
      ; Do we have an active weapon?
      (`/Engine/EditorBlueprintResources/StandardMacros.IsValid` _active_weapon
        (:`Is Valid`
          (bind (_weapondata_name _weapondata_firerate _weapondata_maxcapacity) (break `/Game/ProjectLutr/Blueprints/Data/F_WeaponData` (`/Game/ProjectLutr/Blueprints/BP_WeaponBase.WeaponData` _active_weapon)))
          ; Find How much ammo is needed to reload fully
          (bind _output_get (set `self.NeededAmmo` (- _weapondata_maxcapacity (`/Game/ProjectLutr/Blueprints/BP_WeaponBase.CurrentCapacity` _active_weapon))))
          (`KismetSystemLibrary.PrintString` (`KismetStringLibrary.Concat_StrStr` "Needed Ammo = " (`KismetStringLibrary.Conv_DoubleToString` _output_get)))
          ; Do we even need ammo AND Do we even have extra ammo?
          (if (and (> (`self.NeededAmmo`) 0.0) (> (`GDCharacterBase.GetCapacityReserve` _asbp_hero_character) 0.0))
            ; How much ammo can we actually reload?
            (set `self.ReloadAmount` (`KismetMathLibrary.FMin` (`self.NeededAmmo`) (`GDCharacterBase.GetCapacityReserve` _asbp_hero_character)))
            ; Add Reload Amount to current Capacity
            (`/Game/ProjectLutr/Blueprints/BP_WeaponBase.Reload` _active_weapon (+ (`self.ReloadAmount`) (`/Game/ProjectLutr/Blueprints/BP_WeaponBase.CurrentCapacity` _active_weapon)))
            ; Remove Reload Amount from Ammo Reserve Attribute
            (bind _returnvalue (`AbilitySystemBlueprintLibrary.AssignTagSetByCallerMagnitude` (`AbilitySystemComponent.MakeOutgoingSpec` :`self` (`AbilitySystemBlueprintLibrary.GetAbilitySystemComponent` _asbp_hero_character) :`GameplayEffectClass` "/Game/ProjectLutr/Blueprints/GAS/Effects/GE_ConsumeAmmoResreve.GE_ConsumeAmmoResreve_C" :`Level` 1.0) (struct :`TagName` "SetByCallerTags.AmmoCost") (* (`self.ReloadAmount`) -1.0)))
            (`AbilitySystemComponent.BP_ApplyGameplayEffectSpecToSelf` (`AbilitySystemBlueprintLibrary.GetAbilitySystemComponent` _asbp_hero_character) _returnvalue)
            (`self.K2_EndAbility`)))
        (:`Is Not Valid`
          (`KismetSystemLibrary.PrintString` "Active WEapon isnt valid"))))
    (:`CastFailed`
      (`KismetSystemLibrary.PrintString` "Failed Cast to BP Hero"))))