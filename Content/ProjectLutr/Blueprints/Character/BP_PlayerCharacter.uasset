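; Player character that drives jumping, weapons and assignable abilities through the Gameplay Ability System, with test keys and debug prints.
; Z, X or C picks an ability, then 1–3 binds it to a slot or activates that slot by tag.
; OnWeaponFire sends a camera-trace hit as target data in the weapon's gameplay event.
; ReloadWeapon deducts reserve ammo through a set-by-caller effect; the EquipWeapon body is disconnected, leaving equip to an ability tag.
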(event `Key|Five`
  (params (Key :type "Key Structure"))
  (bind _output_weaponname (break `/Game/ProjectLutr/Blueprints/Data/F_WeaponInstance` (`|GetArrayItem` (`self.InventoryWeaponInstances`))))
  (bind (_value _returnvalue) (`BlueprintMapLibrary.Map_Find` (`/Game/ProjectLutr/Blueprints/Data/BP_WeaponData.WeaponMap` (`self.WeaponData`)) _output_weaponname))
  (:`Pressed`
    (`KismetSystemLibrary.PrintString` (`KismetStringLibrary.Concat_StrStr` "Weapon Name: " (`KismetStringLibrary.Conv_NameToString` _output_weaponname)))
    (if _returnvalue
      (`KismetSystemLibrary.PrintString` "Found Weapon in Weapon Data")
      (`KismetSystemLibrary.PrintString` (`KismetStringLibrary.Concat_StrStr` "Fire Weapon Tag Debug String: " (`BlueprintGameplayTagLibrary.GetDebugStringFromGameplayTagContainer` (`.FireWeaponAbiltiyTag_59_6AE930E14F2C660453308DAB73688676` (break `/Game/ProjectLutr/Blueprints/Data/F_WeaponData` _value)))))
      (else
        (`KismetSystemLibrary.PrintString` "Weapon NOT found in Weapon Data")))))

(event `Key|SpaceBar`
  (params (Key :type "Key Structure"))
  ;[0.2708 0.259 0.07053] Jumping
  (:`Pressed`
    (`AbilitySystemComponent.TryActivateAbilitiesByTag` (`AbilitySystemBlueprintLibrary.GetAbilitySystemComponent` null) (`BlueprintGameplayTagLibrary.MakeGameplayTagContainerFromTag` (struct :`TagName` "Ability.Jump")) true)))

(event `Key|Four`
  (params (Key :type "Key Structure"))
  ;[0.2396 0.226 0] Equip Weapon in first slot of Inventory and bind weapon fire event
  (:`Pressed`
    (if (`KismetArrayLibrary.Array_IsNotEmpty` (`self.InventoryWeaponInstances`))
      (`AbilitySystemComponent.TryActivateAbilitiesByTag` (`AbilitySystemBlueprintLibrary.GetAbilitySystemComponent` null) (`BlueprintGameplayTagLibrary.MakeLiteralGameplayTagContainer` (struct :`GameplayTags` (struct :`(TagName` "Test.Ability.EquipWeapon")))) true))))

(event `Key|One`
  (params (Key :type "Key Structure"))
  ;[0.05729 0 0] Ability Slot Testing
  (:`Pressed`
    (if (`self.bTryAssignTag`)
      (set `self.Slot1Tag` (`self.TagToAssign`))
      (set `self.TagToAssign` (struct))
      (`self.AssignAbilityToSlot`)
      (elif (not (== (`self.Slot1Tag`) (`BlueprintGameplayTagLibrary.MakeGameplayTagContainerFromTag` (struct))))
        (`AbilitySystemComponent.TryActivateAbilitiesByTag` (`AbilitySystemBlueprintLibrary.GetAbilitySystemComponent` null) (`self.Slot1Tag`) true)))))

(event `Key|LeftMouseButton`
  (params (Key :type "Key Structure"))
  (bind _active_weapon (`self.Active Weapon`))
  ;[0.2865 0.1373 0] Call Weapon fire on active weapon if there is one
  (:`Pressed`
    (`/Engine/EditorBlueprintResources/StandardMacros.IsValid` _active_weapon
      (:`Is Valid`
        (`/Game/ProjectLutr/Blueprints/BP_WeaponBase.TryFireWeapon` _active_weapon)))))

(event `Key|Two`
  (params (Key :type "Key Structure"))
  ;[0.05729 0 0] Ability Slot Testing
  (:`Pressed`
    (if (`self.bTryAssignTag`)
      (set `self.Slot2Tag` (`self.TagToAssign`))
      (set `self.TagToAssign` (struct))
      (`self.AssignAbilityToSlot`)
      (elif (not (== (`self.Slot2Tag`) (`BlueprintGameplayTagLibrary.MakeGameplayTagContainerFromTag` (struct))))
        (`AbilitySystemComponent.TryActivateAbilitiesByTag` (`AbilitySystemBlueprintLibrary.GetAbilitySystemComponent` null) (`self.Slot2Tag`) true)))))

(event `OnWeaponFire`
  (bind (_returnvalue_location _returnvalue_rotation) (`KismetMathLibrary.BreakTransform` (`SceneComponent.K2_GetComponentToWorld` (`self.Camera`))))
  (bind (_weapondata_name _weapondata_firerate _weapondata_maxcapacity _weapondata_firecapacitycost _weapondata_spread _weapondata_fireweaponabilityclass _weapondata_reloadweaponabilityclass _weapondata_fireweaponabiltiytag) (break `/Game/ProjectLutr/Blueprints/Data/F_WeaponData` (`/Game/ProjectLutr/Blueprints/BP_WeaponBase.WeaponData` (`self.Active Weapon`))))
  ;[0.3125 0.08745 0] On Weapon Fire Event
  (`/Engine/EditorBlueprintResources/StandardMacros.IsValid` (`self.Active Weapon`)
    (:`Is Valid`
      (bind _outhit (`KismetSystemLibrary.LineTraceSingle` _returnvalue_location (* (`KismetMathLibrary.GetForwardVector` _returnvalue_rotation) 999999.0) "TraceTypeQuery3" false (`|MakeArray` self :!type "Actor Object Reference") "ForDuration" true (struct :`R` 1.0 :`A` 1.0) (struct :`G` 1.0 :`A` 1.0) 1.0))
      (`AbilitySystemBlueprintLibrary.SendGameplayEventToActor` (`ActorComponent.GetOwner` (`AbilitySystemBlueprintLibrary.GetAbilitySystemComponent` null)) (`|GetArrayItem` (`BlueprintGameplayTagLibrary.BreakGameplayTagContainer` _weapondata_fireweaponabiltiytag)) (make `GameplayEventData` (struct) self null null null (struct) (struct) (struct) 0.0 (`AbilitySystemBlueprintLibrary.AbilityTargetDataFromHitResult` _outhit))))))

(event `Key|Three`
  (params (Key :type "Key Structure"))
  ;[0.05729 0 0] Ability Slot Testing
  (:`Pressed`
    (if (`self.bTryAssignTag`)
      (set `self.Slot3Tag` (`self.TagToAssign`))
      (set `self.TagToAssign` (struct))
      (`self.AssignAbilityToSlot`)
      (elif (not (== (`self.Slot3Tag`) (`BlueprintGameplayTagLibrary.MakeGameplayTagContainerFromTag` (struct))))
        (`AbilitySystemComponent.TryActivateAbilitiesByTag` (`AbilitySystemBlueprintLibrary.GetAbilitySystemComponent` null) (`self.Slot3Tag`) true)))))

(event `Key|Z`
  (params (Key :type "Key Structure"))
  ;[0.05729 0 0] Ability Slot Testing
  (:`Pressed`
    (set `self.bTryAssignTag` true)
    (set `self.TagToAssign` (`self.AbilityAlphaTag`))
    (set `self.AbilityToGive` (`self.AbilityAlphaClass`))
    (`KismetSystemLibrary.PrintString` "Initiated Assigning Ability Alpha")))

(event `Key|R`
  (params (Key :type "Key Structure")))

(event `Key|X`
  (params (Key :type "Key Structure"))
  ;[0.05729 0 0] Ability Slot Testing
  (:`Pressed`
    (set `self.bTryAssignTag` true)
    (set `self.TagToAssign` (`self.AbilityBetaTag`))
    (set `self.AbilityToGive` (`self.AbilityBetaClass`))
    (`KismetSystemLibrary.PrintString` "Initiated Assigning Ability Beta")))

(event `Key|C`
  (params (Key :type "Key Structure"))
  ;[0.05729 0 0] Ability Slot Testing
  (:`Pressed`
    (set `self.bTryAssignTag` true)
    (set `self.TagToAssign` (`self.AbilityCharlieTag`))
    (set `self.AbilityToGive` (`self.AbilityCharlieClass`))
    (`KismetSystemLibrary.PrintString` "Initiated Assigning Ability Charlie")))

(event `GiveAbility`
  (params (AbilityToGive :type "GameplayAbility Class Reference"))
  (`AbilitySystemComponent.K2_GiveAbility` (`AbilitySystemBlueprintLibrary.GetAbilitySystemComponent` null) AbilityToGive 0 -1))

(event `RemoveAmmoFromReserve`
  (params (ReloadAmount :type "Float (double-precision)"))
  (bind _returnvalue (`AbilitySystemBlueprintLibrary.AssignTagSetByCallerMagnitude` (`AbilitySystemComponent.MakeOutgoingSpec` :`self` (`AbilitySystemBlueprintLibrary.GetAbilitySystemComponent` null) :`GameplayEffectClass` "/Game/ProjectLutr/Blueprints/GAS/Effects/GE_ConsumeAmmoResreve.GE_ConsumeAmmoResreve_C" :`Level` 1.0) (struct :`TagName` "SetByCallerTags.AmmoCost") (* ReloadAmount -1.0)))
  (`AbilitySystemComponent.BP_ApplyGameplayEffectSpecToSelf` (`AbilitySystemBlueprintLibrary.GetAbilitySystemComponent` null) _returnvalue))

(event `Server_UpdateWeaponReference`
  (params (`Active Weapon` :type "/Game/ProjectLutr/Blueprints/BP_WeaponBase Object Reference"))
  (set `self.Active Weapon` `Active Weapon`)
  (`KismetSystemLibrary.PrintString` "Set Active Weaopn"))

(fn `AssignAbilityToSlot`
  (set `self.bTryAssignTag` false)
  (`AbilitySystemComponent.K2_GiveAbility` (`AbilitySystemBlueprintLibrary.GetAbilitySystemComponent` null) (`self.AbilityToGive`) 0 -1)
  (set `self.AbilityToGive` null)
  (`KismetSystemLibrary.PrintString` (`KismetStringLibrary.Concat_StrStr` "Assigned Ability to " "Slot")))

(fn `EquipWeapon`
  (params (WeaponInstance :type "/Game/ProjectLutr/Blueprints/Data/F_WeaponInstance Structure")))

(fn `OnRep_Active Weapon`)

(fn `ReloadWeapon`
  (locals (NeededAmmo :type "Float (double-precision)") (ReloadAmount :type "Float (double-precision)"))
  (bind _active_weapon (`self.Active Weapon`))
  (bind _active_weapon_2 (`self.Active Weapon`))
  (bind (_weapondata_name _weapondata_firerate _weapondata_maxcapacity) (break `/Game/ProjectLutr/Blueprints/Data/F_WeaponData` (`/Game/ProjectLutr/Blueprints/BP_WeaponBase.WeaponData` _active_weapon_2)))
  ; Do we have an active weapon?
  (`/Engine/EditorBlueprintResources/StandardMacros.IsValid` (`self.Active Weapon`)
    (:`Is Valid`
      ; Find How much ammo is needed to reload fully
      (set `local.NeededAmmo` (- _weapondata_maxcapacity (`/Game/ProjectLutr/Blueprints/BP_WeaponBase.CurrentCapacity` _active_weapon_2)))
      ; Do we even need ammo AND Do we even have extra ammo?
      (if (and (> (`local.NeededAmmo`) 0.0) (> (`self.GetCapacityReserve`) 0.0))
        ; How much ammo can we actually reload?
        (set `local.ReloadAmount` (`KismetMathLibrary.FMin` (`local.NeededAmmo`) (`self.GetCapacityReserve`)))
        ; Add Reload Amount to current Capacity
        (`/Game/ProjectLutr/Blueprints/BP_WeaponBase.Reload` _active_weapon (+ (`local.ReloadAmount`) (`/Game/ProjectLutr/Blueprints/BP_WeaponBase.CurrentCapacity` _active_weapon)))
        ; Remove Reload Amount from Ammo Reserve Attribute
        (bind _returnvalue (`AbilitySystemBlueprintLibrary.AssignTagSetByCallerMagnitude` (`AbilitySystemComponent.MakeOutgoingSpec` :`self` (`AbilitySystemBlueprintLibrary.GetAbilitySystemComponent` null) :`GameplayEffectClass` "/Game/ProjectLutr/Blueprints/GAS/Effects/GE_ConsumeAmmoResreve.GE_ConsumeAmmoResreve_C" :`Level` 1.0) (struct :`TagName` "SetByCallerTags.AmmoCost") (* (`local.ReloadAmount`) -1.0)))
        (`AbilitySystemComponent.BP_ApplyGameplayEffectSpecToSelf` (`AbilitySystemBlueprintLibrary.GetAbilitySystemComponent` null) _returnvalue)))))

(fn `UserConstructionScript`)