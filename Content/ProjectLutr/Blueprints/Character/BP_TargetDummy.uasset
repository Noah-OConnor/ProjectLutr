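; BP_TargetDummy is a target dummy with an Ability System Component and a floating status bar widget component.
; Each tick it rotates the status bar to face the first player controller's view point.
; Logic to bind the WBP_FloatingStatusBar widget to the ability system's attributes exists but is disconnected, and BeginPlay and the construction script are empty.
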(event `self.ReceiveTick`
  (params (DeltaSeconds :type "Float (single-precision)"))
  (bind _returnvalue (`GameplayStatics.GetPlayerController` 0))
  (`/Engine/EditorBlueprintResources/StandardMacros.IsValid` _returnvalue
    (:`Is Valid`
      (`SceneComponent.K2_SetWorldRotation` (`self.UIFloatingStatusBarComponent`) (`KismetMathLibrary.MakeRotFromX` (- (`Controller.GetPlayerViewPoint` _returnvalue) (`SceneComponent.K2_GetComponentLocation` (`self.UIFloatingStatusBarComponent`)))) false false))))

(event `self.ReceiveBeginPlay`)

(fn `UserConstructionScript`)