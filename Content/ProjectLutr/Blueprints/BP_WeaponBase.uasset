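; BP_WeaponBase is a base weapon that tracks ammo capacity and takes its mesh, material and firing cost from WeaponData.
; Initialize stores data and capacity, applies valid visuals, and broadcasts ammo only when the material is valid.
; TryFireWeapon checks capacity before FireWeapon deducts the cost and calls the ammo and fire events, with no shot logic here.
; Reload overwrites capacity and broadcasts it with a max ammo of zero.
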(fn `FireWeapon`
  (bind (_weapondata_name _weapondata_firerate _weapondata_maxcapacity _weapondata_firecapacitycost) (break `/Game/ProjectLutr/Blueprints/Data/F_WeaponData` (`self.WeaponData`)))
  (set `self.CurrentCapacity` (- (`self.CurrentCapacity`) _weapondata_firecapacitycost))
  (`self.OnCurrentAmmoChanged` (`self.CurrentCapacity`) _weapondata_maxcapacity)
  (`self.OnFireWeapon`))

(fn `Initialize`
  (params (WeaponData :type "/Game/ProjectLutr/Blueprints/Data/F_WeaponData Structure") (CurrentCapacity :type "Float (double-precision)"))
  (bind (_weapondata_name _weapondata_firerate _weapondata_maxcapacity _weapondata_firecapacitycost _weapondata_spread _weapondata_fireweaponabilityclass _weapondata_reloadweaponabilityclass _weapondata_fireweaponabiltiytag _weapondata_reloadweaponabilitytag _weapondata_projectileclass _weapondata_staticmesh _weapondata_material) (break `/Game/ProjectLutr/Blueprints/Data/F_WeaponData` (`self.WeaponData`)))
  (set `self.WeaponData` WeaponData)
  (set `self.CurrentCapacity` CurrentCapacity)
  (`/Engine/EditorBlueprintResources/StandardMacros.IsValid` _weapondata_staticmesh
    (:`Is Valid`
      (`SkeletalMeshComponent.SetSkeletalMeshAsset` (`self.WeaponMesh`) _weapondata_staticmesh))
    (:`Is Not Valid`
      _))
  (`/Engine/EditorBlueprintResources/StandardMacros.IsValid` _weapondata_material
    (:`Is Valid`
      (`PrimitiveComponent.SetMaterial` (`self.WeaponMesh`) 0 _weapondata_material)
      (`self.OnCurrentAmmoChanged` (`self.CurrentCapacity`) _weapondata_maxcapacity))))

(fn `Reload`
  (params (NewCapacity :type "Float (double-precision)"))
  (bind _output_get (set `self.CurrentCapacity` NewCapacity))
  (`self.OnCurrentAmmoChanged` _output_get))

(fn `TryFireWeapon`
  (bind (_weapondata_name _weapondata_firerate _weapondata_maxcapacity _weapondata_firecapacitycost) (break `/Game/ProjectLutr/Blueprints/Data/F_WeaponData` (`self.WeaponData`)))
  (if (>= (`self.CurrentCapacity`) _weapondata_firecapacitycost)
    (`self.FireWeapon`)))

(fn `UserConstructionScript`)