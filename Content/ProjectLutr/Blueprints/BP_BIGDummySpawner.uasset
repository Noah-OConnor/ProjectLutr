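; Spawner actor that keeps a population of BP_TargetDummy actors around its location, up to MaxDummyCount.
; A self-rescheduling timer with a random delay attempts a spawn while the tracked list is below the cap.
; Spawns run only with authority, at a random horizontal offset from the spawner at its height.
; Each dummy's OnCharacterDied event removes it from the list, freeing a slot for replacement.
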(event `self.ReceiveBeginPlay`
  (`self.ScheduleNextSpawn`))

(event `ScheduleNextSpawn`
  (`KismetSystemLibrary.K2_SetTimerDelegate` (delegate `TrySpawnDummy`) (`KismetMathLibrary.RandomFloatInRange` 1.0 3.0)))

(event `TrySpawnDummy`
  (if (< (`KismetArrayLibrary.Array_Length` (`self.SpawnedDummies`)) (`self.MaxDummyCount`))
    (`self.SpawnDummy`))
  (`self.ScheduleNextSpawn`))

(event `OnCharacterDied_Event`
  (params (Character :type "LutrCharacterBase Object Reference"))
  (`KismetArrayLibrary.Array_RemoveItem` (`self.SpawnedDummies`) Character))

(event `SpawnDummy`
  (bind _returnvalue (`self.GetTransform`))
  (if (`self.HasAuthority`)
    (bind _returnvalue_2 (`|SpawnActorFromClass` "/Game/ProjectLutr/Blueprints/Character/BP_TargetDummy.BP_TargetDummy_C" (`KismetMathLibrary.MakeTransform` (`KismetMathLibrary.MakeVector` (+ (.x (.location _returnvalue)) (`KismetMathLibrary.RandomFloatInRange` -1000.0 1000.0)) (+ (.y (.location _returnvalue)) (`KismetMathLibrary.RandomFloatInRange` -1000.0 1000.0)) (.z (.location _returnvalue))) (.rotation _returnvalue) (.scale _returnvalue)) "Undefined" "MultiplyWithRoot" null null))
    (`KismetArrayLibrary.Array_Add` (`self.SpawnedDummies`) _returnvalue_2)
    (add `LutrCharacterBase.OnCharacterDied` _returnvalue_2 (delegate `OnCharacterDied_Event`))))

(fn `UserConstructionScript`)